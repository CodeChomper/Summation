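; BP_Die is a die actor that turns green while it detects a neighbor beside it.
; The construction script picks its mesh from DieValue by Value, and BeginPlay creates a dynamic tint material.
; Each Tick sets green or white from Active, then CheckNeighbors refreshes Active for the next frame.
; CheckNeighbors chains short object-type line traces along world ±X and ±Y, stopping at the first hit, with +Y traced twice.
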(event `self.ReceiveBeginPlay`
  (`parent.ReceiveBeginPlay`)
  (bind _returnvalue (`PrimitiveComponent.CreateDynamicMaterialInstance` (`self.StaticMesh`) 0 "/Game/Models/ImphenziaPixPal_001_Tint.ImphenziaPixPal_001_Tint" "None"))
  (set `self.MaterialInst` _returnvalue))

(event `self.ReceiveTick`
  (params (DeltaSeconds :type "Float (single-precision)"))
  (`parent.ReceiveTick` DeltaSeconds)
  (if (`self.Active`)
    (`MaterialInstanceDynamic.SetVectorParameterValue` (`self.MaterialInst`) "Tint" (struct :`G` 0.484375 :`B` 0.003319 :`A` 1.0))
    (else
      (`MaterialInstanceDynamic.SetVectorParameterValue` (`self.MaterialInst`) "Tint" (struct :`R` 1.0 :`G` 1.0 :`B` 1.0 :`A` 1.0))))
  (`self.CheckNeighbors`))

(fn `CheckNeighbors`
  (bind _returnvalue (`SceneComponent.K2_GetComponentLocation` (`self.DefaultSceneRoot`)))
  (bind (_outhit _returnvalue_2) (`KismetSystemLibrary.LineTraceSingleForObjects` _returnvalue (+ _returnvalue (100.0 0.0 0.0)) (`|MakeArray` "ObjectTypeQuery7" :!type "EObjectTypeQuery Enum")))
  (if _returnvalue_2
    (set `self.Active` true)
    (else
      (bind (_outhit_2 _returnvalue_3) (`KismetSystemLibrary.LineTraceSingleForObjects` _returnvalue (+ _returnvalue (-100.0 0.0 0.0)) (`|MakeArray` "ObjectTypeQuery7" :!type "EObjectTypeQuery Enum")))
      (if _returnvalue_3
        (set `self.Active` true)
        (else
          (bind (_outhit_3 _returnvalue_4) (`KismetSystemLibrary.LineTraceSingleForObjects` _returnvalue (+ _returnvalue (0.0 100.0 0.0)) (`|MakeArray` "ObjectTypeQuery7" :!type "EObjectTypeQuery Enum")))
          (if _returnvalue_4
            (set `self.Active` true)
            (else
              (bind (_outhit_4 _returnvalue_5) (`KismetSystemLibrary.LineTraceSingleForObjects` _returnvalue (+ _returnvalue (0.0 100.0 0.0)) (`|MakeArray` "ObjectTypeQuery7" :!type "EObjectTypeQuery Enum")))
              (if _returnvalue_5
                (set `self.Active` true)
                (else
                  (bind (_outhit_5 _returnvalue_6) (`KismetSystemLibrary.LineTraceSingleForObjects` _returnvalue (+ _returnvalue (0.0 -100.0 0.0)) (`|MakeArray` "ObjectTypeQuery7" :!type "EObjectTypeQuery Enum")))
                  (if _returnvalue_6
                    (set `self.Active` true)
                    (else
                      (set `self.Active` false))))))))))))

(fn `UserConstructionScript`
  (`parent.UserConstructionScript`)
  (`StaticMeshComponent.SetStaticMesh` (`self.StaticMesh`) (`|GetArrayItem` (`self.DieValue`) (`self.Value`))))