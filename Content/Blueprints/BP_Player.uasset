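; Player for a grid-based block-pushing game, stepping along X and Y through Enhanced Input.
; Tick interpolates the root toward TargetLocation and allows new moves only once it arrives.
; Each move line-traces one cell ahead: open space sets the new target, while non-block obstacles stop it.
; A BP_MoveableBlock receives a directional push call, and the player advances only if that call returns false.
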(event `self.ReceiveBeginPlay`
  (bind _defaultsceneroot (`self.DefaultSceneRoot`))
  (bind (_returnvalue_x _returnvalue_y) (`KismetMathLibrary.BreakVector` (`SceneComponent.K2_GetComponentLocation` _defaultsceneroot)))
  (`SceneComponent.K2_SetWorldLocation` _defaultsceneroot (`KismetMathLibrary.MakeVector` _returnvalue_x _returnvalue_y 50.5) false false)
  (set `self.TargetLocation` (`SceneComponent.K2_GetComponentLocation` _defaultsceneroot))
  (`EnhancedInputSubsystemInterface.AddMappingContext` (pcsubsystem `EnhancedInputLocalPlayerSubsystem` (`GameplayStatics.GetPlayerController` 0)) "/Game/Blueprints/Input/BP_MC_PlayerControls.BP_MC_PlayerControls" 0 (struct)))

(event `self.ReceiveTick`
  (params (DeltaSeconds :type "Float (single-precision)"))
  (bind _returnvalue (`SceneComponent.K2_GetComponentLocation` (`self.DefaultSceneRoot`)))
  (`SceneComponent.K2_SetWorldLocation` (`self.DefaultSceneRoot`) (`KismetMathLibrary.VInterpTo` _returnvalue (`self.TargetLocation`) DeltaSeconds 20.0) true false)
  (if (== _returnvalue (`self.TargetLocation`))
    (set `self.CanMove` true)
    (else
      (set `self.CanMove` false))))

(event `EnhancedInput|/Game/Blueprints/Input/BP_IA_MoveVert`
  (params (ActionValue :type "Float (double-precision)") (ElapsedSeconds :type "Float (double-precision)") (TriggeredSeconds :type "Float (double-precision)") (InputAction :type "InputAction Object Reference" :default "/Game/Blueprints/Input/BP_IA_MoveVert.BP_IA_MoveVert"))
  (bind _returnvalue (`SceneComponent.K2_GetComponentLocation` (`self.DefaultSceneRoot`)))
  (bind _returnvalue_2 (+ _returnvalue (`KismetMathLibrary.MakeVector` (* ActionValue 100.0))))
  (:`Triggered`
    (if (`self.CanMove`)
      (bind _outhit (`KismetSystemLibrary.LineTraceSingle` _returnvalue _returnvalue_2 "TraceTypeQuery1"))
      (bind (_bblockinghit _binitialoverlap _time _distance _location _impactpoint _normal _impactnormal _physmat _hitactor) (`GameplayStatics.BreakHitResult` _outhit))
      (if _bblockinghit
        (bind _asbp_moveable_block (cast `/Game/Blueprints/BP_MoveableBlock` _hitactor))
        (if (> ActionValue 0.0)
          (bind _isblocked (`/Game/Blueprints/BP_BlockBase.PushedUp` _asbp_moveable_block))
          (if (not _isblocked)
            (set `self.TargetLocation` _returnvalue_2 :!label _label))
          (else
            (bind _isblocked_2 (`/Game/Blueprints/BP_BlockBase.PushedDown` _asbp_moveable_block))
            (if (not _isblocked_2)
              (goto _label))))
        (else
          (set `self.TargetLocation` _returnvalue_2))))))

(event `EnhancedInput|/Game/Blueprints/Input/BP_IA_MoveHorz`
  (params (ActionValue :type "Float (double-precision)") (ElapsedSeconds :type "Float (double-precision)") (TriggeredSeconds :type "Float (double-precision)") (InputAction :type "InputAction Object Reference" :default "/Game/Blueprints/Input/BP_IA_MoveHorz.BP_IA_MoveHorz"))
  (bind _returnvalue (`SceneComponent.K2_GetComponentLocation` (`self.DefaultSceneRoot`)))
  (bind _returnvalue_2 (+ _returnvalue (`KismetMathLibrary.MakeVector` 0.0 (* ActionValue 100.0))))
  (:`Triggered`
    (if (`self.CanMove`)
      (bind _outhit (`KismetSystemLibrary.LineTraceSingle` _returnvalue _returnvalue_2 "TraceTypeQuery1"))
      (bind (_bblockinghit _binitialoverlap _time _distance _location _impactpoint _normal _impactnormal _physmat _hitactor) (`GameplayStatics.BreakHitResult` _outhit))
      (if _bblockinghit
        (bind _asbp_moveable_block (cast `/Game/Blueprints/BP_MoveableBlock` _hitactor))
        (if (> ActionValue 0.0)
          (bind _isblocked (`/Game/Blueprints/BP_BlockBase.PushedRight` _asbp_moveable_block))
          (if (not _isblocked)
            (set `self.TargetLocation` _returnvalue_2 :!label _label_2))
          (else
            (bind _isblocked_2 (`/Game/Blueprints/BP_BlockBase.PushedLeft` _asbp_moveable_block))
            (if (not _isblocked_2)
              (goto _label_2))))
        (else
          (set `self.TargetLocation` _returnvalue_2))))))

(fn `UserConstructionScript`)