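; BP_SummoningTarget is a spawn point that summons a requested number of BP_Enemy actors one after another in the puzzle game.
; SpawnEnemies sets the count, and Tick spawns the next enemy below the target only while its box holds no enemies.
; A timeline raises each enemy toward a fixed height with a vector slerp, playing the spawn sound every update.
; When the last rise finishes, it clears SpawningEnemies on BP_PuzzleGameMode.
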(event `self.ReceiveTick`
  (params (DeltaSeconds :type "Float (single-precision)"))
  (bind _returnvalue (`self.GetTransform`))
  (if (and (> (`self.EnemiesToSpawn`) 0) (== (`self.CubesInSpawn`) 0))
    (bind _returnvalue_2 (`|SpawnActorFromClass` "/Game/Blueprints/BP_Enemy.BP_Enemy_C" (`KismetMathLibrary.MakeTransform` (`KismetMathLibrary.MakeVector` (.x (.location _returnvalue)) (.y (.location _returnvalue)) (- (.z (.location _returnvalue)) 100.0))) "AdjustIfPossibleButAlwaysSpawn" "MultiplyWithRoot" null null))
    (`/Engine/EditorBlueprintResources/StandardMacros.DecrementInt` (`self.EnemiesToSpawn`)
      (:`  `
        (bind (_direction _alpha) (`Timeline|Timeline` :!via `PlayFromStart`)
          (:`Update`
            (bind (_returnvalue_x _returnvalue_y _returnvalue_z) (`KismetMathLibrary.BreakVector` (`self.K2_GetActorLocation` _returnvalue_2)))
            (`self.K2_SetActorLocation` _returnvalue_2 (`KismetMathLibrary.Vector_SlerpNormals` (`KismetMathLibrary.MakeVector` _returnvalue_x _returnvalue_y _returnvalue_z) (`KismetMathLibrary.MakeVector` _returnvalue_x _returnvalue_y 50.0) _alpha) false false)
            (`GameplayStatics.PlaySound2D` "/Game/Sounds/EnemySpawnSound.EnemySpawnSound" 1.0 2.0 0.0 null null))
          (:`Finished`
            (if (== (`self.EnemiesToSpawn`) 0)
              (bind _asbp_puzzle_game_mode (cast `/Game/Blueprints/Lifecycle/BP_PuzzleGameMode` (`GameplayStatics.GetGameMode`)))
              (set `/Game/Blueprints/Lifecycle/BP_PuzzleGameMode.SpawningEnemies` false _asbp_puzzle_game_mode))))))))

(event `SpawnEnemies`
  (params (EnemiesToSpawn :type Integer))
  (set `self.EnemiesToSpawn` EnemiesToSpawn))

(event `self.Box.OnComponentBeginOverlap`
  (params (OverlappedComponent :type "PrimitiveComponent Object Reference") (OtherActor :type "Actor Object Reference") (OtherComp :type "PrimitiveComponent Object Reference") (OtherBodyIndex :type Integer) (bFromSweep :type Boolean) (SweepResult :type "HitResult Structure (by ref)"))
  ;[1 1 1] Track Cubes On Spawn
  (cast `/Game/Blueprints/BP_Enemy` OtherActor)
  (`/Engine/EditorBlueprintResources/StandardMacros.IncrementInt` (`self.CubesInSpawn`)))

(event `self.Box.OnComponentEndOverlap`
  (params (OverlappedComponent :type "PrimitiveComponent Object Reference") (OtherActor :type "Actor Object Reference") (OtherComp :type "PrimitiveComponent Object Reference") (OtherBodyIndex :type Integer))
  ;[1 1 1] Track Cubes On Spawn
  (cast `/Game/Blueprints/BP_Enemy` OtherActor)
  (`/Engine/EditorBlueprintResources/StandardMacros.DecrementInt` (`self.CubesInSpawn`)))

(fn `GetGamePlayTags`
  (returns (GamePlayTags :type "GameplayTagContainer Structure"))
  (return (`self.GamePlayTag`)))

(fn `UserConstructionScript`)