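; BP_Laser is a laser actor built around a Cylinder component that becomes a physics object shortly after spawning.
; BeginPlay waits briefly, then enables physics simulation on the Cylinder.
; The Cylinder's hit event is empty, and the construction script does nothing.
; Disconnected name-check logic for destroying the actor and playing a laser sound, filtering out player and floor names, never runs.
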(event `self.ReceiveBeginPlay`
  (`KismetSystemLibrary.Delay` 0.1)
  (`PrimitiveComponent.SetSimulatePhysics` (`self.Cylinder`) true))

(event `self.Cylinder.OnComponentHit`
  (params (HitComponent :type "PrimitiveComponent Object Reference") (OtherActor :type "Actor Object Reference") (OtherComp :type "PrimitiveComponent Object Reference") (NormalImpulse :type "Vector Structure") (Hit :type "HitResult Structure (by ref)")))

(fn `UserConstructionScript`)