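; BP_Spikes is a spike obstacle that moves up and down automatically on a repeating timer.
; A looping two-second timer flips SpikesDown and plays a sound on every toggle except the first.
; Tick uses VInterpTo to ease the spikes between two absolute world heights, moving faster toward the lower one.
; SpikesDown being true targets the higher position, opposite to what its name suggests.
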(event `self.ReceiveBeginPlay`
  (`KismetSystemLibrary.K2_SetTimerDelegate` (delegate `ToggleSpikes`) 2.0 true))

(event `ToggleSpikes`
  (bind _isa (`/Engine/EditorBlueprintResources/StandardMacros.FlipFlop`)
    (:`A`
      _)
    (:`B`
      _))
  (set `self.SpikesDown` _isa)
  (if (`self.FirstPlayOfSound`)
    (set `self.FirstPlayOfSound` false)
    (else
      (`AudioComponent.Play` (`self.SpikeSound`) 0.0))))

(event `self.ReceiveTick`
  (params (DeltaSeconds :type "Float (single-precision)"))
  (bind _spikes (`self.Spikes`))
  (bind _returnvalue (`SceneComponent.K2_GetComponentLocation` (`self.Spikes`)))
  (bind _x (.x _returnvalue))
  (bind _y (.y _returnvalue))
  (if (`self.SpikesDown`)
    (`SceneComponent.K2_SetWorldLocation` _spikes (`KismetMathLibrary.VInterpTo` _returnvalue (`KismetMathLibrary.MakeVector` _x _y 0.0) DeltaSeconds 10.0) false false)
    (else
      (`SceneComponent.K2_SetWorldLocation` _spikes (`KismetMathLibrary.VInterpTo` _returnvalue (`KismetMathLibrary.MakeVector` _x _y -200.0) DeltaSeconds 50.0) false false))))

(fn `UserConstructionScript`)