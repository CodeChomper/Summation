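; Puzzle game mode that turns active dice totals into enemy waves and decides when a level is complete.
; Each tick sums active BP_Die values for the HUD, and a rise triggers spawning at the next summoning target, selected by numbered actor tag.
; Completion requires reaching BP_LevelSetup's goal with no enemies left or spawning pending, then plays a HUD animation and loads the next level.
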(event `self.ReceiveBeginPlay`
  (bind _outactors (`GameplayStatics.GetAllActorsOfClass` "/Game/Blueprints/BP_Die.BP_Die_C"))
  (set `self.NewVar` _outactors)
  (bind _asbp_hud_player (cast `/Game/Blueprints/UI/Hud/BP_HudPlayer` (`PlayerController.GetHUD` (`GameplayStatics.GetPlayerController` 0))))
  (set `self.HudPlayer` _asbp_hud_player)
  (bind _outactors_2 (`GameplayStatics.GetAllActorsOfClass` "/Game/Blueprints/BP_SummoningTarget.BP_SummoningTarget_C"))
  (set `self.AllTargetPOints` _outactors_2)
  (bind _returnvalue (`GameplayStatics.GetActorOfClass` "/Game/Blueprints/BP_LevelSetup.BP_LevelSetup_C"))
  (bind _output_get (set `self.Level Goal` (`/Game/Blueprints/BP_LevelSetup.LevelGoal` _returnvalue)))
  (`KismetSystemLibrary.DelayUntilNextTick`)
  (`/Game/Blueprints/UI/Hud/BP_HudPlayer.SetLevelGoal` (`self.HudPlayer`) _output_get))

(event `self.ReceiveTick`
  (params (DeltaSeconds :type "Float (single-precision)"))
  (bind _currsum (`self.CurrSum`))
  (bind _levelcomplete (`self.CheckLevelComplete`))
  (if _levelcomplete
    (`|DoOnceMultiInput`
      (:`A Out`
        (`/Game/Blueprints/UI/Hud/CBP_MainHud.PlayLevelCompleteAnimation` (`/Game/Blueprints/UI/Hud/BP_HudPlayer.HudWidget` (`self.HudPlayer`)))
        (`KismetSystemLibrary.Delay` 3.0)
        (message `/Game/Blueprints/Lifecycle/BPI_GameInstance.LoadNextLevel` (`GameplayStatics.GetGameInstance`))))
    (else
      (set `self.CurrSum` 0)
      (for _array_element (`self.NewVar`)
        (if (`/Game/Blueprints/BP_Die.Active` _array_element)
          (set `self.CurrSum` (+ (`self.CurrSum`) (`/Game/Blueprints/BP_BlockBase.Value` _array_element)))))
      (`/Game/Blueprints/UI/Hud/BP_HudPlayer.SetSum` (`self.HudPlayer`) _currsum)
      (if (< (`self.PrevSum`) _currsum)
        (set `self.SpawningEnemies` true)
        (`KismetSystemLibrary.Delay` 0.2)
        (`self.SpawnMonsters`)
        (set `self.PrevSum` _currsum)))))

(event `SpawnMonsters`
  (for _array_element (`self.AllTargetPOints`)
    (if (`self.ActorHasTag` _array_element (`KismetStringLibrary.Conv_StringToName` (`KismetStringLibrary.Conv_IntToString` (`self.SummonLocation`))))
      (set `self.CurSummonTarget` _array_element)
      (`/Engine/EditorBlueprintResources/StandardMacros.IncrementInt` (`self.SummonLocation`)
        (:`  `
          (break)))))
  (set `self.SpawnedEnemies` 0)
  (`/Game/Blueprints/BP_SummoningTarget.SpawnEnemies` (`self.CurSummonTarget`) (`self.CurrSum`)))

(fn `CheckLevelComplete`
  (returns (LevelComplete :type Boolean))
  (bind _outactors (`GameplayStatics.GetAllActorsOfClass` "/Game/Blueprints/BP_Enemy.BP_Enemy_C"))
  (return (and (== (`KismetArrayLibrary.Array_Length` _outactors) 0) (>= (`self.CurrSum`) (`self.Level Goal`)) (not (`self.SpawningEnemies`)))))

(fn `UserConstructionScript`)