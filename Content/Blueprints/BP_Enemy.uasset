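; BP_Enemy is an AI-controlled enemy that moves in 100-unit grid steps and can push BP_MoveableBlock actors.
; MoveVert and MoveHorz line-trace ahead, stop at other obstacles, and step into a block's space only when its directional push call returns false.
; Tick interpolates toward the target with sweep after a short spawn delay, setting the Blackboard's CanMove true only upon arrival to gate further moves.
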(event `self.ReceiveBeginPlay`
  (set `self.Blackboard` (`AIBlueprintHelperLibrary.GetBlackboard` (`AIBlueprintHelperLibrary.GetAIController` self)))
  (`KismetSystemLibrary.K2_SetTimerDelegate` (delegate `SpawnCompleted`) 0.2))

(event `SpawnCompleted`
  (set `self.SpawnComplete` true)
  (set `self.TargetLocation` (`SceneComponent.K2_GetComponentLocation` (`self.DefaultSceneRoot`))))

(event `self.ReceiveTick`
  (params (DeltaSeconds :type "Float (single-precision)"))
  (bind _blackboard (`self.Blackboard`))
  (bind _returnvalue (`SceneComponent.K2_GetComponentLocation` (`self.DefaultSceneRoot`)))
  (if (`self.SpawnComplete`)
    (`SceneComponent.K2_SetWorldLocation` (`self.DefaultSceneRoot`) (`KismetMathLibrary.VInterpTo` _returnvalue (`self.TargetLocation`) DeltaSeconds 20.0) true false)
    (if (== _returnvalue (`self.TargetLocation`))
      (bind _output_get (set `self.CanMove` true))
      (`BlackboardComponent.SetValueAsBool` _blackboard "CanMove" _output_get)
      (else
        (bind _output_get_2 (set `self.CanMove` false))
        (`BlackboardComponent.SetValueAsBool` _blackboard "CanMove" _output_get_2)))))

(event `MoveVert`
  (params (UpOrDown :type "Float (double-precision)"))
  (bind _returnvalue (`SceneComponent.K2_GetComponentLocation` (`self.DefaultSceneRoot`)))
  (bind _returnvalue_2 (+ _returnvalue (`KismetMathLibrary.MakeVector` (* UpOrDown 100.0))))
  (if (`self.CanMove`)
    (bind _outhit (`KismetSystemLibrary.LineTraceSingle` _returnvalue _returnvalue_2 "TraceTypeQuery1"))
    (bind (_bblockinghit _binitialoverlap _time _distance _location _impactpoint _normal _impactnormal _physmat _hitactor) (`GameplayStatics.BreakHitResult` _outhit))
    (if _bblockinghit
      (bind _asbp_moveable_block (cast `/Game/Blueprints/BP_MoveableBlock` _hitactor))
      (if (> UpOrDown 0.0)
        (bind _isblocked (`/Game/Blueprints/BP_BlockBase.PushedUp` _asbp_moveable_block false))
        (if (not _isblocked)
          (set `self.TargetLocation` _returnvalue_2 :!label _label))
        (else
          (bind _isblocked_2 (`/Game/Blueprints/BP_BlockBase.PushedDown` _asbp_moveable_block false))
          (if (not _isblocked_2)
            (goto _label))))
      (else
        (set `self.TargetLocation` _returnvalue_2)))))

(event `MoveHorz`
  (params (RightOrLeft :type "Float (double-precision)"))
  (bind _returnvalue (`SceneComponent.K2_GetComponentLocation` (`self.DefaultSceneRoot`)))
  (bind _returnvalue_2 (+ _returnvalue (`KismetMathLibrary.MakeVector` 0.0 (* RightOrLeft 100.0))))
  (if (`self.CanMove`)
    (bind _outhit (`KismetSystemLibrary.LineTraceSingle` _returnvalue _returnvalue_2 "TraceTypeQuery1"))
    (bind (_bblockinghit _binitialoverlap _time _distance _location _impactpoint _normal _impactnormal _physmat _hitactor) (`GameplayStatics.BreakHitResult` _outhit))
    (if _bblockinghit
      (bind _asbp_moveable_block (cast `/Game/Blueprints/BP_MoveableBlock` _hitactor))
      (if (> RightOrLeft 0.0)
        (bind _isblocked (`/Game/Blueprints/BP_BlockBase.PushedRight` _asbp_moveable_block false))
        (if (not _isblocked)
          (set `self.TargetLocation` _returnvalue_2 :!label _label_2))
        (else
          (bind _isblocked_2 (`/Game/Blueprints/BP_BlockBase.PushedLeft` _asbp_moveable_block false))
          (if (not _isblocked_2)
            (goto _label_2))))
      (else
        (set `self.TargetLocation` _returnvalue_2)))))

(fn `UserConstructionScript`)