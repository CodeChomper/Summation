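; Pushable grid block that slides one tile along the world X or Y axis when one of its four directional Pushed functions is called.
; Each function line-traces one tile ahead and recursively pushes any block found there, so whole rows move unless something else blocks the chain.
; Functions return true when blocked; otherwise they set TargetLocation, which Tick interpolates toward with a swept move.
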(event `self.ReceiveBeginPlay`
  (`parent.ReceiveBeginPlay`)
  (set `self.TargetLocation` (`SceneComponent.K2_GetComponentLocation` (`self.DefaultSceneRoot`))))

(event `self.ReceiveTick`
  (params (DeltaSeconds :type "Float (single-precision)"))
  (`parent.ReceiveTick` DeltaSeconds)
  (`SceneComponent.K2_SetWorldLocation` (`self.DefaultSceneRoot`) (`KismetMathLibrary.VInterpTo` (`SceneComponent.K2_GetComponentLocation` (`self.DefaultSceneRoot`)) (`self.TargetLocation`) DeltaSeconds 20.0) true false))

(fn `PushedDown`
  (returns (IsBlocked :type Boolean))
  (bind _returnvalue (`SceneComponent.K2_GetComponentLocation` (`self.DefaultSceneRoot`)))
  (bind _returnvalue_2 (+ _returnvalue (-100.0 0.0 0.0)))
  (bind _outhit (`KismetSystemLibrary.LineTraceSingle` _returnvalue _returnvalue_2 "TraceTypeQuery1"))
  (bind (_bblockinghit _binitialoverlap _time _distance _location _impactpoint _normal _impactnormal _physmat _hitactor) (`GameplayStatics.BreakHitResult` _outhit))
  (if _bblockinghit
    (bind _asbp_moveable_block (cast `/Game/Blueprints/BP_MoveableBlock` _hitactor)
      (:`then`
        (bind _isblocked (`self.PushedDown` _asbp_moveable_block))
        (if _isblocked
          (return true)
          (else
            (set `self.TargetLocation` _returnvalue_2)
            (return false))))
      (:`CastFailed`
        (return true)))
    (else
      (set `self.TargetLocation` _returnvalue_2)
      (return false))))

(fn `PushedLeft`
  (returns (IsBlocked :type Boolean))
  (bind _returnvalue (`SceneComponent.K2_GetComponentLocation` (`self.DefaultSceneRoot`)))
  (bind _returnvalue_2 (+ _returnvalue (0.0 -100.0 0.0)))
  (bind _outhit (`KismetSystemLibrary.LineTraceSingle` _returnvalue _returnvalue_2 "TraceTypeQuery1"))
  (bind (_bblockinghit _binitialoverlap _time _distance _location _impactpoint _normal _impactnormal _physmat _hitactor) (`GameplayStatics.BreakHitResult` _outhit))
  (if _bblockinghit
    (bind _asbp_moveable_block (cast `/Game/Blueprints/BP_MoveableBlock` _hitactor)
      (:`then`
        (bind _isblocked (`self.PushedLeft` _asbp_moveable_block))
        (if _isblocked
          (return true)
          (else
            (set `self.TargetLocation` _returnvalue_2)
            (return false))))
      (:`CastFailed`
        (return true)))
    (else
      (set `self.TargetLocation` _returnvalue_2)
      (return false))))

(fn `PushedRight`
  (returns (IsBlocked :type Boolean))
  (bind _returnvalue (`SceneComponent.K2_GetComponentLocation` (`self.DefaultSceneRoot`)))
  (bind _returnvalue_2 (+ _returnvalue (0.0 100.0 0.0)))
  (bind _outhit (`KismetSystemLibrary.LineTraceSingle` _returnvalue _returnvalue_2 "TraceTypeQuery1"))
  (bind (_bblockinghit _binitialoverlap _time _distance _location _impactpoint _normal _impactnormal _physmat _hitactor) (`GameplayStatics.BreakHitResult` _outhit))
  (if _bblockinghit
    (bind _asbp_moveable_block (cast `/Game/Blueprints/BP_MoveableBlock` _hitactor)
      (:`then`
        (bind _isblocked (`self.PushedRight` _asbp_moveable_block))
        (if _isblocked
          (return true)
          (else
            (set `self.TargetLocation` _returnvalue_2)
            (return false))))
      (:`CastFailed`
        (return true)))
    (else
      (set `self.TargetLocation` _returnvalue_2)
      (return false))))

(fn `PushedUp`
  (returns (IsBlocked :type Boolean))
  (bind _returnvalue (`SceneComponent.K2_GetComponentLocation` (`self.DefaultSceneRoot`)))
  (bind _returnvalue_2 (+ _returnvalue (100.0 0.0 0.0)))
  (bind _outhit (`KismetSystemLibrary.LineTraceSingle` _returnvalue _returnvalue_2 "TraceTypeQuery1"))
  (bind (_bblockinghit _binitialoverlap _time _distance _location _impactpoint _normal _impactnormal _physmat _hitactor) (`GameplayStatics.BreakHitResult` _outhit))
  (if _bblockinghit
    (bind _asbp_moveable_block (cast `/Game/Blueprints/BP_MoveableBlock` _hitactor)
      (:`then`
        (bind _isblocked (`self.PushedUp` _asbp_moveable_block))
        (if _isblocked
          (return true)
          (else
            (set `self.TargetLocation` _returnvalue_2)
            (return false))))
      (:`CastFailed`
        (return true)))
    (else
      (set `self.TargetLocation` _returnvalue_2)
      (return false))))

(fn `UserConstructionScript`
  (`parent.UserConstructionScript`))